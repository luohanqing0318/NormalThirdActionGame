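; Base player character with an Advanced Locomotion System-style movement model, handling move, look, jump, crouch, walk toggle and sprint input.
; Input and movement callbacks set gait, stance and movement state, while Tick computes speed and acceleration.
; When grounded, data-table settings by rotation mode and stance set max speed, and a curve over gait-mapped speed drives acceleration, braking and friction.
; BPI getters expose this state, with several fields still placeholders.
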(event Collision|EventActorBeginOverlap
  (params (OtherActor :type Actor%20Object%20Reference)))

(event EventTick
  (params (DeltaSeconds :type Float%20%28single-precision%29)))

(event EventBeginPlay
  (|CallParentFunction)
  (CallFunction|OnBeginPlay))

(event EventOnStartCrouch
  (params (HalfHeightAdjust :type Float%20%28single-precision%29) (ScaledHalfHeightAdjust :type Float%20%28single-precision%29))
  ;[1 1 1] 设置蹲伏逻辑
  (|CallParentFunction HalfHeightAdjust ScaledHalfHeightAdjust)
  (Variables|Default|SetStance "NewEnumerator1"))

(event EventOnEndCrouch
  (params (HalfHeightAdjust :type Float%20%28single-precision%29) (ScaledHalfHeightAdjust :type Float%20%28single-precision%29))
  ;[1 1 1] 设置蹲伏逻辑
  (|CallParentFunction HalfHeightAdjust ScaledHalfHeightAdjust)
  (Variables|Default|SetStance "NewEnumerator0"))

(event EventOnMovementModeChanged
  (params (PrevMovementMode :type EMovementMode%20Enum :default "MOVE_None") (NewMovementMode :type EMovementMode%20Enum :default "MOVE_None") (PrevCustomMode :type Byte :default 0) (NewCustomMode :type Byte :default 0))
  ;[1 1 1] 设置跳跃逻辑
  (|CallParentFunction PrevMovementMode NewMovementMode PrevCustomMode NewCustomMode)
  (switch Utilities|FlowControl|Switch|SwitchonEMovementMode NewMovementMode
    (:MOVE_None
      (Variables|Default|SetMovementState "NewEnumerator1" :!label _label))
    (:MOVE_Walking
      (goto _label))
    (:MOVE_NavWalking
      (goto _label))
    (:MOVE_Falling
      (Variables|Default|SetMovementState "NewEnumerator2"))))

(event Input|ActionEvents|InputActionStanceAction
  (params (Key :type Key%20Structure :default "None"))
  ;[1 1 1] 设置蹲伏逻辑
  (:Pressed
    (Character|Crouch))
  (:Released
    (Character|UnCrouch)))

(event Input|ActionEvents|InputActionJumpAction
  (params (Key :type Key%20Structure :default "None"))
  ;[1 1 1] 设置跳跃逻辑
  (:Pressed
    (switch Utilities|FlowControl|Switch|SwitchonALS_MovementState (Variables|Default|GetMovementState)
      (:NewEnumerator0
        _)
      (:NewEnumerator1
        _))
    (Character|Jump))
  (:Released
    (Character|StopJumping)))

(event Input|ActionEvents|InputActionWalkAction
  (params (Key :type Key%20Structure :default "None"))
  ;[1 1 1] 设置冲刺和行走逻辑
  (:Pressed
    (switch Utilities|FlowControl|Switch|SwitchonALS_Gait (Variables|Default|GetGait)
      (:NewEnumerator0
        (Variables|Default|SetGait "NewEnumerator1"))
      (:NewEnumerator1
        (Variables|Default|SetGait "NewEnumerator0")))))

(event Input|ActionEvents|InputActionSprintAction
  (params (Key :type Key%20Structure :default "None"))
  ;[1 1 1] 设置冲刺和行走逻辑
  (:Pressed
    (Variables|Default|SetGait "NewEnumerator2"))
  (:Released
    (Variables|Default|SetGait "NewEnumerator1")))

(event Input|AxisEvents|InputAxisMoveForward/Backwards
  (params (AxisValue :type Float%20%28single-precision%29))
  (Pawn|Input|AddMovementInput (Math|Vector|GetForwardVector (Math|Rotator|MakeRotator 0.0 0.0 (.yaw (Pawn|GetControlRotation :!class /Script/Engine.Pawn)))) AxisValue false))

(event Input|AxisEvents|InputAxisMoveRight/Left
  (params (AxisValue :type Float%20%28single-precision%29))
  (Pawn|Input|AddMovementInput (Math|Vector|GetRightVector (Math|Rotator|MakeRotator 0.0 0.0 (.yaw (Pawn|GetControlRotation :!class /Script/Engine.Pawn)))) AxisValue false))

(event Input|AxisEvents|InputAxisLookUp/Down
  (params (AxisValue :type Float%20%28single-precision%29))
  (Pawn|Input|AddControllerPitchInput AxisValue))

(event Input|AxisEvents|InputAxisLookLeft/Right
  (params (AxisValue :type Float%20%28single-precision%29))
  (Pawn|Input|AddControllerYawInput AxisValue))

(event EventTick
  (params (DeltaSeconds :type Float%20%28single-precision%29))
  (Utilities|FlowControl|Sequence
    (:then_0
      (CallFunction|SetEssentialValues)
      (switch Utilities|FlowControl|Switch|SwitchonALS_MovementState (Variables|Default|GetMovementState)
        (:NewEnumerator1
          (CallFunction|UpdateCharacterMovement))))
    (:then_1
      (CallFunction|CacheValues))))

(fn ConstructionScript)

(fn UpdateCharacterMovement
  (CallFunction|UpdateDynamicMovementSettings (Variables|Default|GetGait)))

(fn UpdateDynamicMovementSettings
  (params (InGait :type ALS_Gait%20Enum :default "NewEnumerator0"))
  (bind _charactermovement (Variables|Character|GetCharacterMovement))
  (bind _charactermovement_2 (Variables|Character|GetCharacterMovement))
  (Utilities|FlowControl|Sequence
    (:then_0
      (Variables|Default|SetCurrentMovementSettings (CallFunction|GetTargetMovementSettings))
      (bind _output_get (Variables|/Script/Engine.CharacterMovementComponent|SetMaxWalkSpeed _charactermovement (Utilities|Select :Index InGait :NewEnumerator0 (.walkspeed (Variables|Default|GetCurrentMovementSettings)) :NewEnumerator1 (.runspeed (Variables|Default|GetCurrentMovementSettings)) :NewEnumerator2 (.sprintspeed (Variables|Default|GetCurrentMovementSettings)))))
      (Variables|/Script/Engine.CharacterMovementComponent|SetMaxWalkSpeedCrouched _charactermovement _output_get))
    (:then_1
      (Variables|/Script/Engine.CharacterMovementComponent|SetMaxAcceleration _charactermovement_2 (.x (Math|Curves|GetVectorValue (.movementcurve (Variables|Default|GetCurrentMovementSettings)) (CallFunction|GetMappedSpeed))))
      (Variables|/Script/Engine.CharacterMovementComponent|SetBrakingDecelerationWalking _charactermovement_2 (.y (Math|Curves|GetVectorValue (.movementcurve (Variables|Default|GetCurrentMovementSettings)) (CallFunction|GetMappedSpeed))))
      (Variables|/Script/Engine.CharacterMovementComponent|SetGroundFriction _charactermovement_2 (.z (Math|Curves|GetVectorValue (.movementcurve (Variables|Default|GetCurrentMovementSettings)) (CallFunction|GetMappedSpeed)))))))

(fn OnBeginPlay
  (Utilities|FlowControl|Sequence
    (:then_0
      (Actor|Tick|AddTickPrerequisiteActor (Variables|Character|GetMesh) self))
    (:then_1
      (CallFunction|SetMovementModel))))

(fn SetMovementModel
  (bind _movementmodel (Variables|Default|GetMovementModel))
  (bind _returnvalue (Utilities|GetDataTableRow (.datatable _movementmodel) (.rowname _movementmodel))
    (:then
      (Variables|Default|SetMovementData _returnvalue))))

(fn GetTargetMovementSettings
  (bind _stance (Variables|Default|GetStance))
  (bind _movementdata (Variables|Default|GetMovementData))
  (switch Utilities|FlowControl|Switch|SwitchonALS_RotationMode (Variables|Default|GetRotationMode)
    (:NewEnumerator0
      (switch Utilities|FlowControl|Switch|SwitchonALS_Stance _stance
        (:NewEnumerator0
          (return (.standing (.velocitydirection _movementdata))))
        (:NewEnumerator1
          (return (.crouching (.velocitydirection _movementdata))))))
    (:NewEnumerator1
      (switch Utilities|FlowControl|Switch|SwitchonALS_Stance _stance
        (:NewEnumerator0
          (return (.standing (.lookingdirection _movementdata))))
        (:NewEnumerator1
          (return (.crouching (.lookingdirection _movementdata))))))
    (:NewEnumerator3
      (switch Utilities|FlowControl|Switch|SwitchonALS_Stance _stance
        (:NewEnumerator0
          (return (.standing (.aiming _movementdata))))))))

(fn GetMappedSpeed
  (bind _currentmovementsettings (Variables|Default|GetCurrentMovementSettings))
  (return (select (> (.runspeed _currentmovementsettings) (Variables|Default|GetSpeed)) (Math|Float|MapRangeClamped (Variables|Default|GetSpeed) (.runspeed _currentmovementsettings) (.sprintspeed _currentmovementsettings) 2.0 3.0) (select (> (.walkspeed _currentmovementsettings) (Variables|Default|GetSpeed)) (Math|Float|MapRangeClamped (Variables|Default|GetSpeed) (.walkspeed _currentmovementsettings) (.runspeed _currentmovementsettings) 1.0 2.0) (Math|Float|MapRangeClamped (Variables|Default|GetSpeed) 0.0 (.walkspeed _currentmovementsettings) 0.0 1.0)))))

(fn SetEssentialValues
  (bind _returnvalue (Transformation|GetVelocity))
  (bind _charactermovement (Variables|Character|GetCharacterMovement))
  (Utilities|FlowControl|Sequence
    (:then_0
      (Variables|Default|SetAcceleration (CallFunction|CalAcceleration)))
    (:then_1
      (bind _output_get (Variables|Default|SetSpeed (Math|Vector|VectorLength (Math|Vector|MakeVector (.x _returnvalue) (.y _returnvalue) 0.0))))
      (Variables|Default|SetIsMoving (> _output_get 1.0)))
    (:then_2
      (bind _output_get_2 (Variables|Default|SetMovementAmount (/ (Math|Vector|VectorLength (Pawn|Components|CharacterMovement|GetCurrentAcceleration _charactermovement)) (Class|MovementComponent|GetMaxSpeed _charactermovement))))
      (Variables|Default|SetHasMovementInput (> _output_get_2 0.0)))))

(fn CacheValues
  (Utilities|FlowControl|Sequence
    (:then_0
      (Variables|Default|SetPrevious%20Velocity (Transformation|GetVelocity)))))

(fn CalAcceleration
  (Utilities|FlowControl|Sequence
    (:then_1
      (return (/ (- (Transformation|GetVelocity) (Variables|Default|GetPrevious%20Velocity)) (Utilities|Time|GetWorldDeltaSeconds))))))

(fn BPIGetCurrentStates
  (return "MOVE_None" (Variables|Default|GetMovementState) "NewEnumerator0" "NewEnumerator4" "NewEnumerator0" (Variables|Default|GetGait) (Variables|Default|GetStance) "NewEnumerator0" "NewEnumerator0"))

(fn BPIGetEssentialValues
  (return (Transformation|GetVelocity) (Variables|Default|GetAcceleration) "0, 0, 0" (Variables|Default|GetIsMoving) (Variables|Default|GetHasMovementInput) (Variables|Default|GetSpeed) (Variables|Default|GetMovementAmount) "0, 0, 0" 0.0))